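; Test player controller for placing, clicking and removing towers on BP_Tile actors with the mouse.
; Left click traces from the cursor on Camera, forwards clicks to an occupied tile's tower, or spawns a scaled-down BP_EricaArcher on a spawnable tile.
; Spawned archers join the trace ignore list, so clicks reach the tile beneath.
; Right click traces on Visibility and destroys the tile's tower; both traces draw persistent debug lines.
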(event EventBeginPlay)

(event EventTick
  (params (DeltaSeconds :type Float%20%28single-precision%29)))

(event Input|MouseEvents|LeftMouseButton
  (params (Key :type Key%20Structure :default "None"))
  (bind _returnvalue (Game|GetPlayerController 0))
  (bind (_worldlocation _worlddirection) (Game|Player|ConvertMouseLocationToWorldSpace _returnvalue))
  (:Pressed
    (bind _outhit (Collision|LineTraceByChannel _worldlocation (+ _worldlocation (* _worlddirection 5e+03)) "TraceTypeQuery2" false (Variables|Default|GetActorsToIgnore) "Persistent" true "(R=1.000000,G=0.000000,B=0.000000,A=1.000000)" "(R=0.115363,G=0.000000,B=1.000000,A=1.000000)"))
    (bind _asbp_tile (Utilities|Casting|CastToBP_Tile (.HitActor (Collision|BreakHitResult _outhit))))
    (Variables|Default|SetLastTileClicked _asbp_tile)
    (if (Class|TileBase|GetOccupied _asbp_tile)
      (Default|GotClicked (Variables|/Game/Test/BP_Tile.BP_Tile_C|GetTower (Variables|Default|GetLastTileClicked)))
      (elif (Class|TileBase|GetTileSpawnable (Variables|Default|GetLastTileClicked))
        (bind _returnvalue_2 (Game|SpawnActorfromClass "/Game/Blueprints/Characters/EricaArcher/BP_EricaArcher.BP_EricaArcher_C" (Math|Transform|MakeTransform (Transformation|GetWorldLocation (Variables|/Script/Engine.Actor|GetRootComponent (Variables|Default|GetLastTileClicked))) "0, 0, 0" "0.500000,0.500000,0.500000") "Undefined" 0 0.0 0))
        (Variables|/Game/Blueprints/Characters/EricaArcher/BP_Tower.BP_Tower_C|SetTileOnSpawned _returnvalue_2 (Variables|Default|GetLastTileClicked))
        (Utilities|Array|Add (Variables|Default|GetActorsToIgnore) _returnvalue_2)
        (Default|TowerSpawned (Variables|Default|GetLastTileClicked) _returnvalue_2)))))

(event Input|MouseEvents|RightMouseButton
  (params (Key :type Key%20Structure :default "None"))
  (bind _returnvalue (Game|GetPlayerController 0))
  (bind (_worldlocation _worlddirection) (Game|Player|ConvertMouseLocationToWorldSpace _returnvalue))
  (:Pressed
    (bind _outhit (Collision|LineTraceByChannel _worldlocation (+ _worldlocation (* _worlddirection 5e+03)) "TraceTypeQuery1" false (Variables|Default|GetActorsToIgnore) "Persistent" true "(R=1.000000,G=0.000000,B=0.851412,A=1.000000)"))
    (bind _asbp_tile (Utilities|Casting|CastToBP_Tile (.HitActor (Collision|BreakHitResult _outhit))))
    (Utilities|IsValid (Variables|/Game/Test/BP_Tile.BP_Tile_C|GetTower _asbp_tile)
      (:Is%20Valid
        (Default|TowerDestroy _asbp_tile)
        (Actor|DestroyActor (Variables|/Game/Test/BP_Tile.BP_Tile_C|GetTower _asbp_tile))))))

(fn ConstructionScript)