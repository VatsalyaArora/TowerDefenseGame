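; Grid tile Blueprint that acts as a tower spawn point, tracking spawnable and occupied state and swapping materials to show changes.
; Enabling it opens a timed placement window, which closes with a notification if the tile is still unoccupied.
; Spawning a tower marks it occupied and switches its nav modifier to a tower area.
; Destruction restores the default nav area immediately, then frees the tile and signals after a cooldown delay.
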(event Custom|TowerDestroy
  (Class|TileBase|SetTileSpawnable false)
  (Rendering|Material|SetMaterial (Variables|Default|GetStaticMesh) 0 "/Engine/EditorMaterials/WidgetMaterial_Z.WidgetMaterial_Z")
  (Class|NavModifierComponent|SetAreaClass (Variables|Default|GetNavModifier) "/Script/NavigationSystem.NavArea_Default")
  (Utilities|FlowControl|Delay (Class|TileBase|GetTimer))
  (Class|TileBase|SetOccupied false)
  (Rendering|Material|SetMaterial (Variables|Default|GetStaticMesh) 0 "/Engine/EditorMaterials/WidgetMaterial_Current.WidgetMaterial_Current")
  (Default|CallTowerDestroyed self))

(event Custom|TowerSpawned
  (params (TowerPlaced :type BP%20Tower%20Object%20Reference))
  (Variables|Tower|SetTower TowerPlaced)
  (Class|TileBase|SetOccupied true)
  (Class|NavModifierComponent|SetAreaClass (Variables|Default|GetNavModifier) "/Game/Test/NavArea_Tower.NavArea_Tower_C"))

(event Custom|EnableSpawnPoint
  (params (Tile :type BP%20Tile%20Object%20Reference))
  (Rendering|Material|SetMaterial (Variables|Default|GetStaticMesh) 0 "/Engine/EditorMaterials/WidgetMaterial_Y.WidgetMaterial_Y")
  (Class|TileBase|SetTileSpawnable true)
  (Utilities|FlowControl|Delay (Class|TileBase|GetStayTimer))
  (if (not (Class|TileBase|GetOccupied))
    (Default|CallDisableSpawnPoint self)
    (Class|TileBase|SetTileSpawnable false)
    (Rendering|Material|SetMaterial (Variables|Default|GetStaticMesh) 0 "/Engine/EditorMaterials/WidgetMaterial_Current.WidgetMaterial_Current")))

(event EventBeginPlay)

(event Collision|EventActorBeginOverlap
  (params (OtherActor :type Actor%20Object%20Reference)))

(event EventTick
  (params (DeltaSeconds :type Float%20%28single-precision%29)))

(fn ConstructionScript)