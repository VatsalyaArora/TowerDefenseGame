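; BP_Grid manages randomly placed, timed tower spawn points across all BP_Tile actors in the level.
; On BeginPlay it gathers tiles and seeds spawn points, then Tick adds more through a repeating Delay.
; MakeSpawnPoint rerolls for an unused tile while below a cap, sets its enable and stay timers, and binds its events.
; Destroyed-tower or disabled-spawn-point events release the tile and lower the count.
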(event Custom|SpawnPointDisable
  (params (Tile :type BP%20Tile%20Object%20Reference))
  (bind _returnvalue (Utilities|Array|RemoveItem (Variables|Grid|GetTilesWithTowers) Tile))
  (if _returnvalue
    (Math|Integer|DecrementInt (Variables|Grid|GetNTowerSpawned))))

(event Custom|TowerDestroyed
  (params (Tile :type BP%20Tile%20Object%20Reference))
  (bind _returnvalue (Utilities|Array|RemoveItem (Variables|Grid|GetTilesWithTowers) Tile))
  (if _returnvalue
    (Math|Integer|DecrementInt (Variables|Grid|GetNTowerSpawned))))

(event EventBeginPlay
  (bind _outactors (Actor|GetAllActorsOfClass "/Game/Test/BP_Tile.BP_Tile_C"))
  (Variables|Grid|SetAllTiles _outactors)
  (CallFunction|MakeInitialSpawnPoint)
  (Variables|Grid|SetMaxTowerCanSpawned 10))

(event Collision|EventActorBeginOverlap
  (params (OtherActor :type Actor%20Object%20Reference)))

(event EventTick
  (params (DeltaSeconds :type Float%20%28single-precision%29))
  (Utilities|FlowControl|Delay (Variables|Grid|GetTimeToMakeSpawnPoint))
  (CallFunction|MakeSpawnPoint))

(fn ConstructionScript)

(fn SpawnTilesinGrid)

(fn MakeInitialSpawnPoint
  (for _index (range 0 40)
    (CallFunction|MakeSpawnPoint))
  (return))

(fn MakeSpawnPoint
  (if (< (Variables|Grid|GetNTowerSpawned) (Variables|Grid|GetMaxTowerCanSpawned))
    (while (or (Utilities|Array|ContainsItem (Variables|Grid|GetTilesWithTowers) (LocalVariables|GetTileFound)) (not (Utilities|IsValid (LocalVariables|GetTileFound))))
      (bind _output_get (Variables|Grid|SetRandomValue (Math|Random|RandomInteger (Utilities|Array|Length (Variables|Grid|GetAllTiles)))))
      (LocalVariables|SetTileFound (Utilities|Array|Get(acopy) (Variables|Grid|GetAllTiles) _output_get)))
    (EventDispatchers|BindEventtoTowerDestroyed (LocalVariables|GetTileFound) (EventDispatchers|CreateEvent :!event Custom|TowerDestroyed))
    (EventDispatchers|BindEventtoDisableSpawnPoint (LocalVariables|GetTileFound) (EventDispatchers|CreateEvent :!event Custom|SpawnPointDisable))
    (Class|TileBase|SetTimer (LocalVariables|GetTileFound) (Variables|Tile|GetTimeToEnable))
    (Class|TileBase|SetStayTimer (LocalVariables|GetTileFound) (Variables|Tile|GetTimeToDisable))
    (Default|EnableSpawnPoint (LocalVariables|GetTileFound) (LocalVariables|GetTileFound))
    (Math|Integer|IncrementInt (Variables|Grid|GetNTowerSpawned)
      (:%20%20
        (Utilities|Array|Add (Variables|Grid|GetTilesWithTowers) (LocalVariables|GetTileFound))))))