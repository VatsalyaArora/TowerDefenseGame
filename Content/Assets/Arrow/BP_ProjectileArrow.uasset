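; Arrow projectile actor that damages skeleton enemies on impact.
; When its box component hits a BP_SkeletonEnemy, it spawns a half-scale spark particle actor at the hit point and passes its Damage to the enemy's projectile impact call.
; The arrow destroys itself on any hit, whether or not the target is a skeleton.
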(event OnComponentHit(Box)
  (params (HitComponent :type Primitive%20Component%20Object%20Reference) (OtherActor :type Actor%20Object%20Reference) (OtherComp :type Primitive%20Component%20Object%20Reference) (NormalImpulse :type Vector :default "0, 0, 0") (Hit :type Hit%20Result%20Structure%20%28by%20ref%29))
  (bind _asbp_skeleton_enemy (Utilities|Casting|CastToBP_SkeletonEnemy OtherActor)
    (:then
      (Game|SpawnActorfromClass "/Game/Blueprints/VFX/Spawn_Particle.Spawn_Particle_C" (Math|Transform|MakeTransform (.Location (Collision|BreakHitResult Hit)) (Transformation|GetActorRotation) "0.500000,0.500000,0.500000") "Undefined" 0 1.0 "/Game/Blueprints/VFX/P_Sparks_C.P_Sparks_C" 0)
      (Default|CallOnProjectileImpact _asbp_skeleton_enemy (Variables|Default|GetDamage)))
    (:CastFailed
      _))
  (Actor|DestroyActor))

(event EventBeginPlay
  (|CallParentFunction) ; This node is disabled and will not be called.\nDrag off pins to build functionality.
)

(event Collision|EventActorBeginOverlap
  (params (OtherActor :type Actor%20Object%20Reference))
  (|CallParentFunction OtherActor) ; This node is disabled and will not be called.\nDrag off pins to build functionality.
)

(event EventTick
  (params (DeltaSeconds :type Float%20%28single-precision%29))
  (|CallParentFunction DeltaSeconds) ; This node is disabled and will not be called.\nDrag off pins to build functionality.
)

(fn ConstructionScript
  (|CallParentFunction))