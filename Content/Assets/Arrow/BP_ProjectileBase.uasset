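; Base projectile Blueprint in the Arrow assets, providing configurable flight toward a target actor.
; The construction script applies speed and gravity to the ProjectileMovement component and enables homing on the target's root component when a valid target and the homing flag are set.
; RotateToTarget redirects velocity straight at the target at the set speed.
; DoEnemyDamage is an empty function, with no damage logic here.
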(event Custom|RotateToTarget
  (Variables|/Script/Engine.MovementComponent|SetVelocity (Variables|Default|GetProjectileMovement) (* (Math|Vector|GetUnitDirection(Vector) (Transformation|GetActorLocation) (Transformation|GetActorLocation (Variables|Target|GetProjectileTarget))) (Variables|ProjectileSetting|GetSpeed))))

(fn ConstructionScript
  (bind _projectilemovement (Variables|Default|GetProjectileMovement))
  (bind _projectilemovement_2 (Variables|Default|GetProjectileMovement))
  (Variables|/Script/Engine.ProjectileMovementComponent|SetInitialSpeed _projectilemovement (Variables|ProjectileSetting|GetSpeed))
  (Variables|/Script/Engine.ProjectileMovementComponent|SetMaxSpeed _projectilemovement (Variables|ProjectileSetting|GetSpeed))
  (Variables|/Script/Engine.ProjectileMovementComponent|SetProjectileGravityScale _projectilemovement (Variables|ProjectileSetting|GetGravity))
  (Variables|Target|GetProjectileTarget
    (:then
      (if (Variables|ProjectileSetting|GetIsHoming)
        (Variables|/Script/Engine.ProjectileMovementComponent|SetbIsHomingProjectile _projectilemovement_2 true)
        (Variables|/Script/Engine.ProjectileMovementComponent|SetHomingTargetComponent _projectilemovement_2 (Variables|/Script/Engine.Actor|GetRootComponent (Variables|Target|GetProjectileTarget)))))
    (:else)))

(fn DoEnemyDamage)