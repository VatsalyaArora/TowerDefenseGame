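; Player controller that places and clicks Erica archer units on the landscape and switches the camera between two fixed views.
; BeginPlay caches the level's CameraActor and Landscape.
; A left click traces under the cursor, calling GotClicked on a hit archer or spawning a new one at a fixed height on landscape hits.
; W and S snap the camera to preset transforms on opposite sides of the field.
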(event EventBeginPlay
  (bind _returnvalue (Actor|GetActorOfClass "/Script/Engine.CameraActor"))
  (Variables|Default|SetCameraActor _returnvalue)
  (bind _returnvalue_2 (Actor|GetActorOfClass "/Script/Landscape.Landscape"))
  (Variables|Default|SetLandscape _returnvalue_2))

(event EventTick
  (params (DeltaSeconds :type Float%20%28single-precision%29)))

(event Input|MouseEvents|LeftMouseButton
  (params (Key :type Key%20Structure :default "None"))
  (bind _returnvalue (Game|GetPlayerController 0))
  (bind (_worldlocation _worlddirection) (Game|Player|ConvertMouseLocationToWorldSpace _returnvalue))
  (:Pressed
    (bind _outhit (Collision|LineTraceByChannel _worldlocation (+ _worldlocation (* _worlddirection 5e+03)) "TraceTypeQuery1" false 0 "None"))
    (bind _asbp_erica_archer (Utilities|Casting|CastToBP_EricaArcher (.HitActor (Collision|BreakHitResult _outhit)))
      (:then
        (Default|GotClicked _asbp_erica_archer))
      (:CastFailed
        (if (== (.HitActor (Collision|BreakHitResult _outhit)) (Variables|Default|GetLandscape))
          (Game|SpawnActorfromClass "/Game/Blueprints/Characters/EricaArcher/BP_EricaArcher.BP_EricaArcher_C" (Math|Transform|MakeTransform (Math|Vector|MakeVector (.x (.Location (Collision|BreakHitResult _outhit))) (.y (.Location (Collision|BreakHitResult _outhit))) 2e+02) "0,-90.000000,0.000000") "Undefined" 0 1e+01 0))))))

(event Input|KeyboardEvents|W
  (params (Key :type Key%20Structure :default "None"))
  (:Pressed
    (Transformation|SetActorTransform (Variables|Default|GetCameraActor) (Math|Transform|MakeTransform "1500.000000,350.000000,1300.000000" "315.000000,180.000000,0.000000"))))

(event Input|KeyboardEvents|S
  (params (Key :type Key%20Structure :default "None"))
  (:Pressed
    (Transformation|SetActorTransform (Variables|Default|GetCameraActor) (Math|Transform|MakeTransform "-1500.000000,350.000000,1300.000000" "315.000000,0.000000,0.000000"))))

(fn ConstructionScript)