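; Health Blueprint in the AI folder that stores current and maximum health and exposes functions to read, set and reset it.
; BeginPlay resets current health to the maximum.
; TakeDamage subtracts damage without clamping or death handling and prints the result as debug text.
; RegenerateHealth adds health while current is at or below maximum, so it can overshoot, and returns true only once current exceeds maximum.
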(event EventBeginPlay
  (CallFunction|ResetHealth))

(fn TakeDamage
  (params (Damage :type Float%20%28double-precision%29))
  (bind _output_get (Variables|Default|SetCurrentHealth (- (Variables|Default|GetCurrentHealth) Damage)))
  (Development|PrintString (Utilities|String|ToString(Float) _output_get) true true "(R=0.000000,G=1.000000,B=0.137491,A=1.000000)"))

(fn GetHealth
  (return (Variables|Default|GetCurrentHealth)))

(fn RegenerateHealth
  (params (AddedValue :type Float%20%28double-precision%29))
  (if (>= (Variables|Default|GetMaxHealth) (Variables|Default|GetCurrentHealth))
    (Variables|Default|SetCurrentHealth (+ AddedValue (Variables|Default|GetCurrentHealth)))
    (return false)
    (else
      (return true))))

(fn SetMaxHealth
  (params (NewHealth :type Float%20%28double-precision%29))
  (Variables|Default|SetMaxHealth NewHealth))

(fn SetHealth
  (params (NewHealth :type Float%20%28double-precision%29))
  (Variables|Default|SetCurrentHealth NewHealth))

(fn ResetHealth
  (Variables|Default|SetCurrentHealth (Variables|Default|GetMaxHealth)))