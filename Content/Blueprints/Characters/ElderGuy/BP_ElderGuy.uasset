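; BP_ElderGuy is an AI-controlled defender that tracks nearby skeleton enemies and destroys itself when its tower-died event fires.
; Sphere overlaps maintain an enemy queue, which feeds the Blackboard along with the animation instance, queue size and death flag.
; Tick keeps the skeleton mesh just above its ground-range component and checks health.
; Crossing health thresholds triggers Chaos master fields and smoke to break its geometry collection in stages.
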(event OnComponentBeginOverlap(Sphere)
  (params (OverlappedComponent :type Primitive%20Component%20Object%20Reference) (OtherActor :type Actor%20Object%20Reference) (OtherComp :type Primitive%20Component%20Object%20Reference) (OtherBodyIndex :type Integer) (bFromSweep :type Boolean) (SweepResult :type Hit%20Result%20Structure%20%28by%20ref%29))
  ;[1 1 1] Left for Enemy Overlap
  (bind _asbp_skeleton_enemy (Utilities|Casting|CastToBP_SkeletonEnemy OtherActor))
  (Class|EnemyQueue|AddEnemy (Variables|Default|GetEnemyQueue) _asbp_skeleton_enemy))

(event OnComponentEndOverlap(Sphere)
  (params (OverlappedComponent :type Primitive%20Component%20Object%20Reference) (OtherActor :type Actor%20Object%20Reference) (OtherComp :type Primitive%20Component%20Object%20Reference) (OtherBodyIndex :type Integer))
  (bind _asbp_skeleton_enemy (Utilities|Casting|CastToBP_SkeletonEnemy OtherActor))
  (Class|EnemyQueue|RemoveEnemy (Variables|Default|GetEnemyQueue) _asbp_skeleton_enemy))

(event Custom|Tower%20Is%20Dead
  (Actor|DestroyActor))

(event EventBeginPlay
  (|CallParentFunction)
  (Variables|Default|SetAmountDamage 35.0)
  (Utilities|FlowControl|Sequence
    (:then_0
      (bind _asfs_master_field (Utilities|Casting|CastToFS_MasterField (Variables|/Script/Engine.ChildActorComponent|GetChildActor (Variables|Default|GetFS_MasterField))))
      (Utilities|Array|Add (Variables|Default|GetMaster%20Field) _asfs_master_field)
      (bind _asfs_master_field_2 (Utilities|Casting|CastToFS_MasterField (Variables|/Script/Engine.ChildActorComponent|GetChildActor (Variables|Default|GetFS_MasterField1))))
      (Utilities|Array|Add (Variables|Default|GetMaster%20Field) _asfs_master_field_2))
    (:then_1
      (AI|Components|Blackboard|SetValueasObject (AI|GetBlackboard (AI|GetAIController self)) (Utilities|Name|MakeLiteralName "EnemyQueue") (Variables|Default|GetEnemyQueue))
      (bind _asabp_elder_guy (Utilities|Casting|CastToABP_ElderGuy (Components|SkeletalMesh|GetAnimInstance (Variables|Default|GetSkeleton))))
      (AI|Components|Blackboard|SetValueasObject (AI|GetBlackboard (AI|GetAIController self)) (Utilities|Name|MakeLiteralName "ABP") _asabp_elder_guy))
    (:then_2
      (EventDispatchers|BindEventtoTowerDied (delegate Custom|Tower%20Is%20Dead)))))

(event EventTick
  (params (DeltaSeconds :type Float%20%28single-precision%29))
  (bind _skeleton (Variables|Default|GetSkeleton))
  (bind _returnvalue (Transformation|GetWorldLocation _skeleton))
  (|CallParentFunction DeltaSeconds)
  (Utilities|FlowControl|Sequence
    (:then_0
      (Transformation|SetWorldLocation _skeleton (Math|Vector|MakeVector (.x _returnvalue) (.y _returnvalue) (+ (.z (Transformation|GetWorldLocation (Variables|Default|GetGroundRange))) 5e+01)) true false))
    (:then_1
      (CallFunction|CheckHealth))
    (:then_2
      (bind _returnvalue_2 (Class|EnemyQueue|GetQueueSize (Variables|Default|GetEnemyQueue)))
      (Class|BlackboardComponent|SetValueasInt (AI|GetBlackboard (AI|GetAIController self)) (Utilities|Name|MakeLiteralName "EnemyQueueSize") _returnvalue_2))))

(fn ConstructionScript
  (|CallParentFunction))

(fn CheckHealth
  (bind _health (Variables|Default|GetHealth))
  (bind _health_percentage_counter (Variables|Default|GetHealth%20Percentage%20Counter))
  (bind _health_2 (Default|GetHealth (Variables|Default|GetHealth)))
  (if (<= _health_2 0.0)
    (AI|Components|Blackboard|SetValueasBool (AI|GetBlackboard (AI|GetAIController self)) (Utilities|Name|MakeLiteralName "IsDead") true)
    (else
      (bind _health_3 (Default|GetHealth _health))
      (if (and (< _health_3 (- (Variables|/Game/Blueprints/AI/Health.Health_C|GetMaxHealth _health) (* (Variables|Default|GetHealth%20Percentage%20Counter) 50))) (< (Variables|Default|GetHealth%20Percentage%20Counter) 3))
        (CallFunction|EffectsonDamage _health_percentage_counter)
        (Math|Integer|IncrementInt _health_percentage_counter)))))

(fn EffectsonDamage
  (params (HealthCounter :type Integer))
  (bind _returnvalue (Transformation|GetActorTransform))
  (bind _returnvalue_2 (- HealthCounter 1))
  (bind (_location _rotation) (Math|Transform|BreakTransform _returnvalue))
  (Default|CETrigger (Utilities|Array|Get(acopy) (Variables|Default|GetMaster%20Field) _returnvalue_2))
  (Game|SpawnActorfromClass "/Game/Blueprints/VFX/Spawn_Particle.Spawn_Particle_C" (Math|Transform|MakeTransform _location _rotation "0.500000,0.500000,0.500000") "Undefined" 0 0.6 "/Game/Realistic_Starter_VFX_Pack_Vol2/Particles/Smoke/P_Smoke_C.P_Smoke_C" 0)
  (if (== _returnvalue_2 (Utilities|Array|Length (Variables|Default|GetMaster%20Field)))
    (Collision|SetCollisionObjectType (Variables|Default|GetGeometryCollection) "ECC_WorldStatic")))