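; Erica archer defender that automatically shoots skeleton enemies entering its detection sphere.
; Overlaps feed EnemyQueue; Tick locks the queue's last enemy and starts the attack animation.
; The AnimBP's Damage flag times each shot, which spawns a targeted arrow, applies damage directly and turns the mesh toward surviving targets.
; Lost health progressively destroys pedestal components as a visual health gauge, and zero health destroys the actor.
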(event OnComponentBeginOverlap(Sphere)
  (params (OverlappedComponent :type Primitive%20Component%20Object%20Reference) (OtherActor :type Actor%20Object%20Reference) (OtherComp :type Primitive%20Component%20Object%20Reference) (OtherBodyIndex :type Integer) (bFromSweep :type Boolean) (SweepResult :type Hit%20Result%20Structure%20%28by%20ref%29))
  ;[1 1 1] Left for Enemy Overlap
  (bind _asbp_skeleton_enemy (Utilities|Casting|CastToBP_SkeletonEnemy OtherActor))
  (Class|EnemyQueue|AddEnemy (Variables|Default|GetEnemyQueue) _asbp_skeleton_enemy)
  (Variables|Default|SetStart%20Attacking true))

(event OnComponentEndOverlap(Sphere)
  (params (OverlappedComponent :type Primitive%20Component%20Object%20Reference) (OtherActor :type Actor%20Object%20Reference) (OtherComp :type Primitive%20Component%20Object%20Reference) (OtherBodyIndex :type Integer))
  (bind _asbp_skeleton_enemy (Utilities|Casting|CastToBP_SkeletonEnemy OtherActor))
  (Class|EnemyQueue|RemoveEnemy (Variables|Default|GetEnemyQueue) _asbp_skeleton_enemy))

(event EventBeginPlay
  (|CallParentFunction)
  (Variables|Default|SetPedestalArray (Utilities|Array|MakeArray (Variables|Default|GetPedestal0) (Variables|Default|GetPedestal1) (Variables|Default|GetPedestal2) (Variables|Default|GetPedestal3) (Variables|Default|GetPedestal4) (Variables|Default|GetPedestal5))))

(event EventTick
  (params (DeltaSeconds :type Float%20%28single-precision%29))
  (Utilities|FlowControl|Sequence
    (:then_0
      (if (Variables|Default|GetStart%20Attacking)
        (CallFunction|GetTarget)
        (CallFunction|Attack)))
    (:then_1
      (CallFunction|CheckHealth))))

(fn ConstructionScript)

(fn Attack
  (bind _currentenemy (Variables|Default|GetCurrentEnemy))
  (bind _health (Variables|/Game/Blueprints/Characters/SkeletonZombie/BP_SkeletonEnemy.BP_SkeletonEnemy_C|GetHealth _currentenemy))
  (if (Variables|Default|GetIsEnemyLocked)
    (Utilities|IsValid (Variables|Default|GetCurrentEnemy)
      (:Is%20Valid
        (bind _asabp_erica_archer (Utilities|Casting|CastToABP_EricaArcher (Components|SkeletalMesh|GetAnimInstance (Variables|Default|GetSkeleton))))
        (if (Variables|/Game/Blueprints/ABP/EricaArcher/ABP_EricaArcher.ABP_EricaArcher_C|GetDamage _asabp_erica_archer)
          (Variables|/Game/Blueprints/ABP/EricaArcher/ABP_EricaArcher.ABP_EricaArcher_C|SetDamage _asabp_erica_archer false)
          (CallFunction|SpawnArrow)
          (Default|TakeDamage _health 1e+01)
          (bind _health_2 (Default|GetHealth _health))
          (if (<= _health_2 0.0)
            (Variables|Default|SetIsEnemyLocked false)
            (Class|EnemyQueue|RemoveEnemy (Variables|Default|GetEnemyQueue) (Variables|Default|GetCurrentEnemy))
            (else
              (CallFunction|LookTowardsEnemy)))))
      (:Is%20Not%20Valid
        (Variables|Default|SetIsEnemyLocked false)))))

(fn GetTarget
  (if (not (Variables|Default|GetIsEnemyLocked))
    (bind _returnvalue (Class|EnemyQueue|GetLastEnemy (Variables|Default|GetEnemyQueue)))
    (bind _asbp_skeleton_enemy (Utilities|Casting|CastToBP_SkeletonEnemy _returnvalue))
    (Variables|Default|SetCurrentEnemy _asbp_skeleton_enemy)
    (Variables|Default|SetIsEnemyLocked true)
    (bind _asabp_erica_archer (Utilities|Casting|CastToABP_EricaArcher (Components|SkeletalMesh|GetAnimInstance (Variables|Default|GetSkeleton))))
    (Variables|/Game/Blueprints/ABP/EricaArcher/ABP_EricaArcher.ABP_EricaArcher_C|SetAttacking _asabp_erica_archer true)))

(fn LookTowardsEnemy
  (Transformation|SetRelativeRotation (Variables|Default|GetSkeleton) (Math|Rotator|MakeRotator 0.0 0.0 (.Yaw (Math|Rotator|BreakRotator (Math|Rotator|FindLookatRotation (Transformation|GetWorldLocation (Variables|Default|GetSkeleton)) (Transformation|GetActorLocation (Variables|Default|GetCurrentEnemy)))))) true false))

(fn CheckHealth
  (bind _health (Variables|Default|GetHealth))
  (Utilities|FlowControl|Sequence
    (:then_0
      (bind _health_2 (Default|GetHealth _health))
      (if (< _health_2 (- (Variables|/Game/Blueprints/AI/Health.Health_C|GetMaxHealth _health) (* (Variables|Default|GetHealthPercentageCounter) 20)))
        (Components|DestroyComponent (Utilities|Array|Get(acopy) (Variables|Default|GetPedestalArray) (- (Variables|Default|GetHealthPercentageCounter) 1)))
        (Math|Integer|IncrementInt (Variables|Default|GetHealthPercentageCounter))))
    (:then_1
      (bind _health_3 (Default|GetHealth _health))
      (if (<= _health_3 0.0)
        (Actor|DestroyActor)))))

(fn SpawnArrow
  (bind _returnvalue (Game|SpawnActorfromClass "/Game/Assets/Arrow/BP_ProjectileArrow.BP_ProjectileArrow_C" (Transformation|GetWorldTransform (Variables|Default|GetProjectileDirection)) "Undefined" 0 1e+03 0.2 false (Variables|Default|GetAmountDamage) 0))
  (Variables|/Game/Assets/Arrow/BP_ProjectileBase.BP_ProjectileBase_C|SetTarget _returnvalue (Variables|Default|GetCurrentEnemy))
  (Default|RotatetoTarget _returnvalue))