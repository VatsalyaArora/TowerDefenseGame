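; Tower actor with a projectile range attack and a toggleable ground range indicator.
; BeginPlay sizes the GroundRange marker and detection sphere from RangeRadius and puts both on a custom collision channel.
; RangeAttack spawns BP_Projectile at the ProjectileDirection transform, and GotClicked toggles the marker's visibility.
; CheckPath is an empty stub, and this Blueprint contains no targeting logic or calls to RangeAttack.
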(event EventBeginPlay
  (bind _rangeradius (Variables|Default|GetRangeRadius))
  (Transformation|SetWorldScale3D (Variables|Default|GetGroundRange) (Math|Vector|MakeVector _rangeradius _rangeradius 0.1))
  (Collision|SetCollisionObjectType (Variables|Default|GetGroundRange) "ECC_GameTraceChannel1")
  (Collision|SetCollisionObjectType (Variables|Default|GetSphere) "ECC_GameTraceChannel1")
  (Components|Sphere|SetSphereRadius (Variables|Default|GetSphere) (* (Variables|Default|GetRangeRadius) 5e+01) true)
  (CallFunction|CheckPath))

(event Collision|EventActorBeginOverlap
  (params (OtherActor :type Actor%20Object%20Reference)))

(event EventTick
  (params (DeltaSeconds :type Float%20%28single-precision%29)))

(fn ConstructionScript)

(fn RangeAttack
  (Game|SpawnActorfromClass "/Game/Blueprints/Projectiles/BP_Projectile.BP_Projectile_C" (Transformation|GetWorldTransform (Variables|Default|GetProjectileDirection)) "Undefined" 0 0))

(fn GotClicked
  (if (Variables|/Script/Engine.SceneComponent|GetbVisible (Variables|Default|GetGroundRange))
    (Rendering|SetVisibility (Variables|Default|GetGroundRange) false false)
    (else
      (Rendering|SetVisibility (Variables|Default|GetGroundRange) true false))))

(fn CheckPath)