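; Skeleton enemy character that seeks and attacks towers and takes damage from projectile impacts.
; Pawn sensing and capsule hits with the archer set Blackboard keys, which Tick clears when the tower becomes invalid.
; Tick also polls Animation Blueprint flags to time tower damage and destroy the actor after death.
; At zero health it starts the death animation and disables collision; reaching heaven removes it and its AI controller.
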(event OnSeePawn(PawnSensing)
  (params (Pawn :type Pawn%20Object%20Reference))
  (bind _self self)
  (bind _returnvalue (AI|GetAIController _self))
  (bind _returnvalue_2 (AI|GetBlackboard _returnvalue))
  (bind _asbp_tower (Utilities|Casting|CastToBP_Tower Pawn))
  (Variables|Default|SetTower _asbp_tower)
  (AI|Components|Blackboard|SetValueasObject _returnvalue_2 (Utilities|Name|MakeLiteralName "Tower") Pawn)
  (AI|Components|Blackboard|SetValueasBool _returnvalue_2 (Utilities|Name|MakeLiteralName "TowerFound") true))

(event OnComponentHit(CapsuleComponent)
  (params (HitComponent :type Primitive%20Component%20Object%20Reference) (OtherActor :type Actor%20Object%20Reference) (OtherComp :type Primitive%20Component%20Object%20Reference) (NormalImpulse :type Vector :default "0, 0, 0") (Hit :type Hit%20Result%20Structure%20%28by%20ref%29))
  (Utilities|Casting|CastToBP_EricaArcher OtherActor)
  (AI|Components|Blackboard|SetValueasBool (AI|GetBlackboard (AI|GetAIController self)) (Utilities|Name|MakeLiteralName "TowerClose") true))

(event Custom|ReachedHeaven
  (Actor|DestroyActor (AI|GetAIController self))
  (Actor|DestroyActor))

(event Custom|ProjectileImpact
  (params (Damage :type Float%20%28double-precision%29))
  (Default|TakeDamage (Variables|Default|GetHealth) Damage))

(event EventBeginPlay
  (Collision|SetCollisionObjectType (Variables|Character|GetMesh) "ECC_GameTraceChannel3")
  (Collision|SetCollisionObjectType (Variables|Collision|GetCapsuleComponent) "ECC_GameTraceChannel3")
  (Default|ResetHealth (Variables|Default|GetHealth))
  (EventDispatchers|BindEventtoEnemyReachedHeaven (delegate Custom|ReachedHeaven))
  (bind _asabp_skeleton_enemy (Utilities|Casting|CastToABP_SkeletonEnemy (Components|SkeletalMesh|GetAnimInstance (Variables|Character|GetMesh))))
  (Variables|Default|SetSkeletonAnimation _asabp_skeleton_enemy)
  (Collision|SetActorEnableCollision true)
  (EventDispatchers|BindEventtoOnProjectileImpact (delegate Custom|ProjectileImpact)))

(event EventTick
  (params (DeltaSeconds :type Float%20%28single-precision%29))
  (Utilities|FlowControl|Sequence
    (:then_0
      (if (Variables|/Game/Blueprints/Characters/SkeletonZombie/ABP_SkeletonEnemy.ABP_SkeletonEnemy_C|GetDead (Variables|Default|GetSkeletonAnimation))
        (Actor|DestroyActor)))
    (:then_1
      (if (not (Variables|/Game/Blueprints/Characters/SkeletonZombie/ABP_SkeletonEnemy.ABP_SkeletonEnemy_C|GetDead (Variables|Default|GetSkeletonAnimation)))
        (CallFunction|CheckHealth)))
    (:then_2
      (CallFunction|CheckTower))
    (:then_3
      (CallFunction|AttackTower (Variables|Default|GetTower)))))

(fn ConstructionScript)

(fn CheckHealth
  (bind _health (Default|GetHealth (Variables|Default|GetHealth)))
  (if (<= _health 0.0)
    (Default|DeadBeginEvent (Variables|Default|GetSkeletonAnimation))
    (AI|Components|Blackboard|SetValueasBool (AI|GetBlackboard (AI|GetAIController self)) (Utilities|Name|MakeLiteralName "IsDead") true)
    (Collision|SetActorEnableCollision false)
    (return true)
    (else
      (return false))))

(fn AttackTower
  (params (Tower :type BP%20Tower%20Object%20Reference))
  (if (Variables|/Game/Blueprints/Characters/SkeletonZombie/ABP_SkeletonEnemy.ABP_SkeletonEnemy_C|GetDamage (Variables|Default|GetSkeletonAnimation))
    (Variables|/Game/Blueprints/Characters/SkeletonZombie/ABP_SkeletonEnemy.ABP_SkeletonEnemy_C|SetDamage (Variables|Default|GetSkeletonAnimation) false)
    (Utilities|IsValid Tower
      (:Is%20Valid
        (bind _health (Default|GetHealth (Variables|/Game/Blueprints/Characters/EricaArcher/BP_Tower.BP_Tower_C|GetHealth Tower)))
        (if (not (<= _health 0.0))
          (Default|TakeDamage (Variables|/Game/Blueprints/Characters/EricaArcher/BP_Tower.BP_Tower_C|GetHealth Tower) 5e+01))))))

(fn CheckTower
  (Utilities|IsValid (Variables|Default|GetTower)
    (:Is%20Not%20Valid
      (Utilities|IsValid (AI|GetBlackboard (AI|GetAIController self))
        (:Is%20Valid
          (AI|Components|Blackboard|SetValueasBool (AI|GetBlackboard (AI|GetAIController self)) (Utilities|Name|MakeLiteralName "TowerFound") false)
          (AI|Components|Blackboard|SetValueasBool (AI|GetBlackboard (AI|GetAIController self)) (Utilities|Name|MakeLiteralName "TowerClose") false)
          (Default|RunBeginEvent (Variables|Default|GetSkeletonAnimation)))))))