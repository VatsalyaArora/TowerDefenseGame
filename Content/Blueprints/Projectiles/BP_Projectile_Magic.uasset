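; Magic fire projectile that explodes on skeleton enemies and applies area damage.
; A box hit on a skeleton triggers a one-time Niagara explosion, hides the fire effect, enlarges the sphere collider and destroys the actor shortly after.
; Sphere overlaps pass damage to each skeleton via CallOnProjectileImpact, with debug prints.
; A delay on Tick destroys the projectile after a few seconds regardless of impact.
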(event OnComponentHit(Box)
  (params (HitComponent :type Primitive%20Component%20Object%20Reference) (OtherActor :type Actor%20Object%20Reference) (OtherComp :type Primitive%20Component%20Object%20Reference) (NormalImpulse :type Vector :default "0, 0, 0") (Hit :type Hit%20Result%20Structure%20%28by%20ref%29))
  (bind _location (Collision|BreakHitResult Hit))
  (Utilities|Casting|CastToBP_SkeletonEnemy OtherActor)
  (if (Variables|Default|GetExplode)
    (Variables|Default|SetExplode false)
    (Niagara|SpawnSystematLocation "/Game/NiagaraSystem/NS_Explosion.NS_Explosion" (Math|Vector|MakeVector (.x _location) (.y _location) (- (.z _location) 1.2e+02)) (Math|Rotator|MakeRotator 0.0 0.0 0.0) "5.000000,5.000000,5.000000")
    (Components|Sphere|SetSphereRadius (Variables|Default|GetSphere) 1e+02 true)
    (Development|SetHiddeninGame (Variables|Default|GetP_ElementalFire_Lg) true false)
    (Utilities|FlowControl|Delay 0.5)
    (Actor|DestroyActor)))

(event OnComponentBeginOverlap(Sphere)
  (params (OverlappedComponent :type Primitive%20Component%20Object%20Reference) (OtherActor :type Actor%20Object%20Reference) (OtherComp :type Primitive%20Component%20Object%20Reference) (OtherBodyIndex :type Integer) (bFromSweep :type Boolean) (SweepResult :type Hit%20Result%20Structure%20%28by%20ref%29))
  (Development|PrintString "damage" true true "(R=0.004252,G=1.000000,B=0.000000,A=1.000000)" 1e+01)
  (bind _asbp_skeleton_enemy (Utilities|Casting|CastToBP_SkeletonEnemy OtherActor))
  (Default|CallOnProjectileImpact _asbp_skeleton_enemy (Variables|Default|GetDamage) self)
  (Development|PrintString (Utilities|String|ToString(Boolean) (Variables|/Game/Blueprints/Characters/SkeletonZombie/BP_SkeletonEnemy.BP_SkeletonEnemy_C|GetTookDamage _asbp_skeleton_enemy))))

(event Collision|EventActorBeginOverlap
  (params (OtherActor :type Actor%20Object%20Reference)))

(event EventTick
  (params (DeltaSeconds :type Float%20%28single-precision%29))
  (Utilities|FlowControl|Delay 3.0)
  (Actor|DestroyActor))

(fn ConstructionScript
  (|CallParentFunction))