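; Resource system Blueprint that manages the coin economy for placing towers.
; It looks up a tower's cost from its class display name, compares it to current coins for affordability, and deducts it when a tower spawns.
; A separate function adds coins, while the event graph and construction script are empty.
; Coin storage and cost lookup rely on functions defined outside these graphs.
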(event EventBeginPlay)

(event Collision|EventActorBeginOverlap
  (params (OtherActor :type Actor%20Object%20Reference)))

(event EventTick
  (params (DeltaSeconds :type Float%20%28single-precision%29)))

(fn ConstructionScript)

(fn IsEnoughResources
  (params (Tower :type Actor%20Class%20Reference))
  (bind _returnvalue (Class|ResourceSystem|ReturnRequiredResources (Utilities|GetClassDisplayName Tower)))
  (return (<= _returnvalue (Class|ResourceSystem|GetCoins))))

(fn IncreaseCoins
  (params (AmountIncreased :type Integer))
  (Class|ResourceSystem|AddCoins AmountIncreased))

(fn TowerSpawned
  (params (TowerClass :type Actor%20Class%20Reference))
  (bind _returnvalue (Class|ResourceSystem|ReturnRequiredResources (Utilities|GetClassDisplayName TowerClass)))
  (Class|ResourceSystem|ReduceCoins _returnvalue)
  (return))